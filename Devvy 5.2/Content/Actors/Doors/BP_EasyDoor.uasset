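; BP_EasyDoor is a door actor that starts an easy level when overlapped.
; If the overlapping actor is BP_Devvy, it sets the easy-level flag and increments the level count in BP_GameInctance.
; A second Sequence branch resets the game instance's Health from the StartHealth row of DT_GameVariables and opens the "Main" level.
; That second branch skips the BP_Devvy check, so any overlapping actor triggers it.
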(event `self.ReceiveActorBeginOverlap`
  (params (OtherActor :type "Actor Object Reference"))
  (`|ExecutionSequence`
    (:`then_0`
      (bind _asbp_game_inctance (cast `/Game/GameInstance/BP_GameInctance` (`GameplayStatics.GetGameInstance`)))
      (cast `/Game/Character/BP_Devvy` OtherActor)
      (set `/Game/GameInstance/BP_GameInctance.IsEasyLevel` true _asbp_game_inctance)
      (`/Engine/EditorBlueprintResources/StandardMacros.IncrementInt` (`/Game/GameInstance/BP_GameInctance.LevelsCurrent` _asbp_game_inctance)))
    (:`then_1`
      (bind _asbp_game_inctance_2 (cast `/Game/GameInstance/BP_GameInctance` (`GameplayStatics.GetGameInstance`)))
      (bind _returnvalue (`|GetDataTableRow` "/Game/DataTables/DT_GameVariables.DT_GameVariables" "StartHealth")
        (:`then`
          (set `/Game/GameInstance/BP_GameInctance.Health` (`.Value_13_0F2E9FFD4556FA13943A45B39CBE4C82` (break `/Game/DataTables/S_GameVariables` _returnvalue)) _asbp_game_inctance_2)
          (`GameplayStatics.OpenLevel` "Main"))))))

(fn `UserConstructionScript`)